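; Procedural-generation actor that paints a heightmap from an array of vertices and exports it to the project directory.
; DrawBrush creates and clears a square render target, then shows it on the Plane through a dynamic material instance.
; It draws a one-pixel canvas box per vertex, scaling X/Y by matrix size and turning absolute Z into brightness via HSV.
; The render target is then exported under the supplied file name with a .png extension.
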(event EventBeginPlay)

(fn ConstructionScript)

(fn DrawBrush
  (params (ArraysVertex :type Array%20of%20Vectors) (MatrixSize :type Integer) (FormatRenderTarget :type ETextureRenderTargetFormat%20Enum :default "RTF_R8") (FileNameToSave :type String))
  (Utilities|FlowControl|Sequence
    (:then_0
      (bind _returnvalue (Rendering|CreateRenderTarget2D MatrixSize MatrixSize FormatRenderTarget))
      (bind _output_get (Variables|Default|SetHeightfieldRT _returnvalue))
      (Rendering|ClearRenderTarget2D _output_get "(R=0.093750,G=0.000000,B=0.000000,A=1.000000)"))
    (:then_1
      (bind _returnvalue_2 (Rendering|Material|CreateDynamicMaterialInstance "/Game/StrategyGame/MaterialLibrary/M_HeightfieldPainte.M_HeightfieldPainte" "None" :!class /Script/Engine.KismetMaterialLibrary))
      (Rendering|Material|SetTextureParameterValue _returnvalue_2 "RenderTarget" (Variables|Default|GetHeightfieldRT))
      (Rendering|Material|SetTextureParameterValue _returnvalue_2 "RenderTarget" 0)
      (Rendering|Material|SetMaterial (Variables|Default|GetPlane) 0 _returnvalue_2))
    (:then_2
      (bind (_canvas _size _context) (Rendering|BeginDrawCanvastoRenderTarget (Variables|Default|GetHeightfieldRT)))
      (for _array_element ArraysVertex
        (Canvas|DrawBox _canvas (Math|Vector2D|MakeVector2D (* MatrixSize (.x _array_element)) (* MatrixSize (.y _array_element))) "(X=1.000000,Y=1.000000)" 0.0 (Class|KismetMathLibrary|HSVtoRGB 0.0 0.0 (Math|Float|Absolute(Float) (.z _array_element)) 1.0)))
      (Rendering|EndDrawCanvastoRenderTarget _context))
    (:then_3
      (Rendering|ExportRenderTarget (Variables|Default|GetHeightfieldRT) (Class|KismetSystemLibrary|GetProjectDirectory) (Utilities|String|Append FileNameToSave "" ".png")))))