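; Procedural landscape actor that builds terrain meshes at runtime from a supplied vertex array.
; CreateLandscapeRuntime builds shared grid triangles (winding set by Top) and UVs, then splits the array into Width×Width components.
; Each component spawns another instance of this actor, as the modulo-1 check always passes, and fills its procedural mesh section.
; Sections receive computed normals and tangents, the painted landscape material, collision and a navmesh update.
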(fn ConstructionScript)

(fn MakeVERTEX
  (params (x :type Integer) (y :type Integer) (width :type Integer))
  (bind _returnvalue (Math|Conversions|ToFloat(Integer) width))
  (bind _returnvalue_2 (/ 1.0 _returnvalue))
  (Utilities|Array|Add (Variables|Default|GetVERTEX) (Math|Vector|MakeVector (* x _returnvalue_2) (* y _returnvalue_2) 0.0)))

(fn MakeTriangles
  (bind _triangles (Variables|Default|GetTRIANGLES))
  (bind _width (Variables|Default|GetWidth))
  (bind _width_2 (Variables|Default|GetWidth))
  (bind _returnvalue (- _width 1))
  (for _index (range 0 (- _width_2 1))
    (for _index_2 (range 0 (- _width_2 1))
      ;[1 1 1] Triangles
      (if (and (!= _returnvalue _index) (!= _index_2 _returnvalue))
        (if (Variables|Default|GetTop)
          (Class|KismetProceduralMeshLibrary|ConvertQuadtoTriangles _triangles (+ _index_2 (* _index (Variables|Default|GetWidth))) (+ 1 (+ _index_2 (* _index (Variables|Default|GetWidth)))) (+ 1 (+ _index_2 (* (+ _index 1) (Variables|Default|GetWidth)))) (+ _index_2 (* (+ _index 1) (Variables|Default|GetWidth))))
          (else
            (Class|KismetProceduralMeshLibrary|ConvertQuadtoTriangles _triangles (+ _index_2 (* (+ _index 1) (Variables|Default|GetWidth))) (+ 1 (+ _index_2 (* (+ _index 1) (Variables|Default|GetWidth)))) (+ 1 (+ _index_2 (* _index (Variables|Default|GetWidth)))) (+ _index_2 (* _index (Variables|Default|GetWidth))))))))))

(fn MakeUV
  (params (UVScale :type Float%20%28single-precision%29))
  (bind _width (Variables|Default|GetWidth))
  (bind _width_2 (Variables|Default|GetWidth))
  (for _index (range 0 (- _width 1))
    (for _index_2 (range 0 (- _width 1))
      ;[1 1 1] UV
      (Utilities|Array|Add (Variables|Default|GetUV) (Math|Vector2D|MakeVector2D (* (* (/ 1.0 (Math|Conversions|ToFloat(Integer) (- _width_2 1))) (Math|Conversions|ToFloat(Integer) _index)) UVScale) (* UVScale (* (/ 1.0 (Math|Conversions|ToFloat(Integer) (- _width_2 1))) (Math|Conversions|ToFloat(Integer) _index_2))))))))

(fn CreateLandscapeRuntime
  (params (vertexArray :type Array%20of%20Vectors) (WidthInComponent :type Integer))
  (Variables|Default|SetVERTEX_0 vertexArray)
  (bind _output_get (Variables|Default|SetWidth WidthInComponent))
  (CallFunction|MakeTriangles)
  (CallFunction|MakeUV (Math|Conversions|ToFloat(Integer) (Variables|Default|GetWidth)))
  (for _index (range 0 (- (/ (Utilities|Array|Length vertexArray) (* _output_get _output_get)) 1))
    (bind _returnvalue (Class|GenerationFun|CreateVertexArrayComponent vertexArray _index (Variables|Default|GetWidth)))
    (Variables|Default|SetVERTEX _returnvalue)
    (bind (_normals _tangents) (Class|KismetProceduralMeshLibrary|CalculateTangentsforMesh (Variables|Default|GetVERTEX) (Variables|Default|GetTRIANGLES) (Variables|Default|GetUV)))
    (if (== (Math|Integer|%(Integer) _index 1) 0)
      (bind _returnvalue_2 (Game|SpawnActorfromClass "BP_ProceduralGenerationLandscape_C" (Transformation|GetActorTransform) "Undefined" 0 0))
      (Variables|Default|SetProceduralMeshComponent (Variables|BP_ProceduralGenerationLandscape_C|GetProceduralMesh _returnvalue_2)))
    (Class|ProceduralMeshComponent|CreateMeshSectionLinearColor (Variables|Default|GetProceduralMeshComponent) _index (Variables|Default|GetVERTEX) (Variables|Default|GetTRIANGLES) _normals (Variables|Default|GetUV) 0 0 0 0 _tangents true)
    (Rendering|Material|SetMaterial (Variables|Default|GetProceduralMeshComponent) _index "/Game/StrategyGame/MaterialLibrary/MI_LandscapePainted.MI_LandscapePainted")
    (Class|ProceduralMeshComponent|AddCollisionConvexMesh (Variables|Default|GetProceduralMeshComponent) (Variables|Default|GetVERTEX))
    (Class|GenerationFun|UpdateNavMeshComponent (Variables|Default|GetProceduralMeshComponent))))