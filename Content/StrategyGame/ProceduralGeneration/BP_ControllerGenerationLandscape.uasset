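; Procedural terrain controller that runs the whole generation pipeline from its Construction Script, configured by enum and parameter settings.
; It builds a vertex array from Diamond-Square, Voronoi, both combined or a file, then optionally applies thermal, hydraulic or equalizing erosion.
; The result feeds a runtime landscape, a heightmap Painter or both.
; Optional steps scatter random trees, save vertices to file and spawn a diagonal row of units.
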(fn ConstructionScript
  (CallFunction|ControllExperiance))

(fn ControllExperiance
  (bind _self self)
  (bind _returnvalue (Transformation|GetActorTransform _self))
  (switch Utilities|FlowControl|Switch|SwitchonEMatrixSize (Variables|DefaultGeneration|GetChooseSizeComponent)
    (:NewEnumerator0
      (Variables|DefaultGeneration|SetSizeOfComponentLandscape 8))
    (:NewEnumerator1
      (Variables|DefaultGeneration|SetSizeOfComponentLandscape 16))
    (:NewEnumerator2
      (Variables|DefaultGeneration|SetSizeOfComponentLandscape 32))
    (:NewEnumerator3
      (Variables|DefaultGeneration|SetSizeOfComponentLandscape 64))
    (:NewEnumerator4
      (Variables|DefaultGeneration|SetSizeOfComponentLandscape 128))
    (:NewEnumerator5
      (Variables|DefaultGeneration|SetSizeOfComponentLandscape 256))
    (:NewEnumerator6
      (Variables|DefaultGeneration|SetSizeOfComponentLandscape 512)))
  (switch Utilities|FlowControl|Switch|SwitchonEMatrixSize (Variables|DefaultGeneration|GetChooseMatrixSize)
    (:NewEnumerator0
      (Variables|DefaultGeneration|SetMatrixSize 8))
    (:NewEnumerator1
      (Variables|DefaultGeneration|SetMatrixSize 16))
    (:NewEnumerator2
      (Variables|DefaultGeneration|SetMatrixSize 32))
    (:NewEnumerator3
      (Variables|DefaultGeneration|SetMatrixSize 64))
    (:NewEnumerator4
      (Variables|DefaultGeneration|SetMatrixSize 128))
    (:NewEnumerator5
      (Variables|DefaultGeneration|SetMatrixSize 256))
    (:NewEnumerator6
      (Variables|DefaultGeneration|SetMatrixSize 512)))
  ;[0.6793 0.6457 1] Step1. Create Base Terrain
  (switch Utilities|FlowControl|Switch|SwitchonEChooseBaseTerrian (Variables|DefaultGeneration|GetchooseBaseTerrain)
    (:NewEnumerator0
      ;;[1 1 1] Diamond-Square
      (bind _returnvalue_2 (Class|ProceduralGenerationActor|DiamondSquareAlgh (Variables|DefaultGeneration|GetMatrixSize) (Variables|Diamond-Square|GetRoughness_0) false))
      (bind _returnvalue_3 (Class|GenerationFun|NormalizeCoordVector _returnvalue_2))
      (Variables|Default|SetVertexArray _returnvalue_3))
    (:NewEnumerator1
      ;;[1 1 1] Voronoi Diagram
      (bind _returnvalue_4 (Class|ProceduralGenerationActor|VoronoiDiagrams (Variables|VoronoiDiagram|Getcoef1) (Variables|VoronoiDiagram|Getcoef2) (Variables|DefaultGeneration|GetMatrixSize) false (Variables|VoronoiDiagram|GetCountHills) (Variables|VoronoiDiagram|GetbDaminMapUse) (Variables|VoronoiDiagram|GetparametrMinus)))
      (bind _returnvalue_5 (Class|GenerationFun|NormalizeCoordVector _returnvalue_4))
      (Variables|Default|SetVertexArray _returnvalue_5))
    (:NewEnumerator2
      ;;[1 1 1] Combination Algh
      (bind _coordvert (CallFunction|CombinationDSandVoronoi))
      (Variables|Default|SetVertexArray _coordvert))
    (:NewEnumerator3
      ;;[1 1 1] Read Frome File
      (bind _vertexarray (Class|GenerationFun|ReadVertexArrayfromFile (Variables|DefaultGeneration|GetInputFile)))
      (Variables|Default|SetVertexArray _vertexarray))
    (:NewEnumerator4
      _))
  ;[0.7094 1 0.6634] Step 2. Modification Terrian
  (switch Utilities|FlowControl|Switch|SwitchonEChooseErosion (Variables|DefaultGeneration|GetchooseErosion)
    (:NewEnumerator0
      ;;[1 0.9114 0.2448] Thermal Erosion
      (for _index (range 1 (Variables|Erosion|GetCountIteration))
        (if (Variables|Erosion|GetbOptimizationThermalErosion)
          (bind _arrayvertout (Class|ProceduralGenerationActor|ThermalErosion (Variables|Erosion|Gettalus) (Variables|Default|GetVertexArray)))
          (Variables|Default|SetVertexArray _arrayvertout)
          (else
            (bind _arrayvertout_2 (Class|ProceduralGenerationActor|OnlyMinThermalErosion (Variables|Erosion|Gettalus) (Variables|Default|GetVertexArray)))
            (Variables|Default|SetVertexArray _arrayvertout_2)))))
    (:NewEnumerator1
      ;;[0.4081 0.7201 1] HydraulicErosin
      (bind _arrayvertout_3 (Class|ProceduralGenerationActor|HydraulicErosion (Variables|Default|GetVertexArray) (Variables|Erosion|GetCountIteration) (Variables|Erosion|GetbOptimizationHydraulicErosion) false))
      (Variables|Default|SetVertexArray _arrayvertout_3))
    (:NewEnumerator2
      ;;[1 0.4948 0.4948] Alghoritm Equalizing
      (for _index_2 (range 1 (Variables|Erosion|GetCountIteration))
        (bind _arrayvertout_4 (Class|ProceduralGenerationActor|ErosionOptAlgh (Variables|Default|GetVertexArray) (Variables|Erosion|Gettalus)))
        (Variables|Default|SetVertexArray _arrayvertout_4)))
    (:NewEnumerator3
      ;;[1 1 1] Two Step of Algoritm Equalizing
      (for _index_3 (range 1 (Variables|Erosion|GetCountIteration))
        (bind _arrayvertout_5 (Class|ProceduralGenerationActor|ErosionOptAlgh (Variables|Default|GetVertexArray) (Variables|Erosion|Gettalus)))
        (Variables|Default|SetVertexArray _arrayvertout_5))
      (for _index_4 (range 1 (Variables|Erosion|GetCountIterationForSecondStepEqualizingAlghoritm))
        (bind _arrayvertout_6 (Class|ProceduralGenerationActor|ErosionOptAlgh (Variables|Default|GetVertexArray) (Variables|Erosion|GettalusForSecondStepEqualizingAlghoritm)))
        (Variables|Default|SetVertexArray _arrayvertout_6)))
    (:NewEnumerator4
      _))
  ;[1 0.6756 0.9048] Step 3. Generation Result
  (switch Utilities|FlowControl|Switch|SwitchonEResultGeneration (Variables|DefaultGeneration|GetresultGeneration)
    (:NewEnumerator0
      (bind _returnvalue_6 (Class|GenerationFun|ChangeVertexArrayCoord (Variables|Default|GetVertexArray) (Variables|DefaultGeneration|GetcoefXY) (Variables|DefaultGeneration|GetcoefZ)))
      (Default|CreateLandscapeRuntime (Variables|Reference|GetProceduralGenerationLandscape) _returnvalue_6 (Variables|DefaultGeneration|GetSizeOfComponentLandscape)))
    (:NewEnumerator2
      (Default|DrawBrush (Variables|Reference|GetPainter) (Variables|Default|GetVertexArray) (Variables|DefaultGeneration|GetMatrixSize) (Variables|DefaultGeneration|GetFormatRenderTarget)))
    (:NewEnumerator1
      (Default|DrawBrush (Variables|Reference|GetPainter) (Variables|Default|GetVertexArray) (Variables|DefaultGeneration|GetMatrixSize) (Variables|DefaultGeneration|GetFormatRenderTarget))
      (bind _returnvalue_7 (Class|GenerationFun|ChangeVertexArrayCoord (Variables|Default|GetVertexArray) (Variables|DefaultGeneration|GetcoefXY) (Variables|DefaultGeneration|GetcoefZ)))
      (Default|CreateLandscapeRuntime (Variables|Reference|GetProceduralGenerationLandscape) _returnvalue_7 (Variables|DefaultGeneration|GetSizeOfComponentLandscape))))
  ;[1 1 1] Create Tree
  (if (Variables|DefaultGeneration|GetbCreateTree)
    (bind _returnvalue_8 (Class|GenerationFun|ChangeVertexArrayCoord (Variables|Default|GetVertexArray) (Variables|DefaultGeneration|GetcoefXY) (Variables|DefaultGeneration|GetcoefZ)))
    (CallFunction|CreateTree _returnvalue_8))
  ;[1 1 1] Save Array Vertex in File
  (if (Variables|Save|GetSaveVertexArrayToFile)
    (for _array_element (Variables|Default|GetVertexArray)
      (bind _returnvalue_9 (Class|GenerationFun|NextString (Utilities|String|Append (Utilities|String|ToString(Float) (.x _array_element)) ";" (Utilities|String|ToString(Float) (.y _array_element)) ";" (Utilities|String|ToString(Float) (.z _array_element)))))
      (Utilities|Array|Add (Variables|Default|GetData) _returnvalue_9))
    (Class|GenerationFun|SaveDatatoFile (Variables|Default|GetData) (Variables|Save|GetNameFile)))
  ;[1 1 1] Create Units
  (if (Variables|DefaultGeneration|GetbSpawnUnits)
    (for _index_5 (range 0 8)
      (Game|SpawnActorfromClass "/Game/StrategyGame/Units/BP_Unit.BP_Unit_C" (Math|Transform|MakeTransform (Math|Vector|MakeVector (+ (.x (.location _returnvalue)) (* _index_5 1e+02) (* (/ (Variables|DefaultGeneration|GetMatrixSize) 2) (Variables|DefaultGeneration|GetcoefXY))) (+ (.y (.location _returnvalue)) (* (/ (Variables|DefaultGeneration|GetMatrixSize) 2) (Variables|DefaultGeneration|GetcoefXY)) (* _index_5 1e+02)) (+ (* (Variables|DefaultGeneration|GetcoefZ) 1.0) (.z (.location _returnvalue)))) (.rotation _returnvalue) (.scale _returnvalue)) "Undefined" 0 0))))

(fn CreateTree
  (params (VertexArray :type Array%20of%20Vectors))
  (bind _returnvalue (Math|Random|RandomRotator false))
  (bind _returnvalue_2 (Class|GenerationFun|CreateTrees VertexArray))
  (for _array_element _returnvalue_2
    (if (> (Math|Random|RandomIntegerinRange 0 100) 98)
      (bind _result (Math|Integer|IncrementInt (LocalVariables|GetcountTree))
        (:%20%20
          (Math|Integer|CompareInt _result 100
            (:>
              (Math|Integer|CompareInt (Math|Random|RandomIntegerinRange 0 1)
                (:>
                  (Game|SpawnActorfromClass "/Game/StrategyGame/ProceduralGeneration/BP_Tree.BP_Tree_C" (Math|Transform|MakeTransform (Math|Vector|MakeVector (.X (Math|Vector|BreakVector _array_element)) (.Y (Math|Vector|BreakVector _array_element)) (- (.Z (Math|Vector|BreakVector _array_element)) 1e+01)) (Math|Rotator|MakeRotator 0.0 0.0 (.yaw _returnvalue)) "1,1,1") "Undefined" 0 0))
                (:==
                  (Game|SpawnActorfromClass "/Game/StrategyGame/ProceduralGeneration/BP_Tree1.BP_Tree1_C" (Math|Transform|MakeTransform (Math|Vector|MakeVector (.X (Math|Vector|BreakVector _array_element)) (.Y (Math|Vector|BreakVector _array_element)) (- (.Z (Math|Vector|BreakVector _array_element)) 1e+01)) (Math|Rotator|MakeRotator 0.0 0.0 (.yaw _returnvalue)) "1,1,1") "Undefined" 0 0))))))))))

(fn CombinationDSandVoronoi
  (bind (_seconds _partialseconds) (Class|GameplayStatics|GetAccurateRealTime))
  (bind (_seconds_2 _partialseconds_2) (Class|GameplayStatics|GetAccurateRealTime))
  (bind _matrixsize (Variables|DefaultGeneration|GetMatrixSize))
  ;[1 1 1] Combination Algh
  (Variables|Default|SetTimeVar (+ (Math|Conversions|ToFloat(Integer) _seconds) _partialseconds))
  (Utilities|FlowControl|Sequence
    (:then_0
      (bind _returnvalue (Class|ProceduralGenerationActor|VoronoiDiagrams (Variables|VoronoiDiagram|Getcoef1) (Variables|VoronoiDiagram|Getcoef2) _matrixsize false (Variables|VoronoiDiagram|GetCountHills) (Variables|VoronoiDiagram|GetbDaminMapUse) (Variables|VoronoiDiagram|GetparametrMinus)))
      (bind _returnvalue_2 (Class|GenerationFun|NormalizeCoordVector _returnvalue)))
    (:then_1
      (bind _returnvalue_3 (Class|ProceduralGenerationActor|DiamondSquareAlgh _matrixsize (Variables|Diamond-Square|GetRoughness_0) false))
      (bind _returnvalue_4 (Class|GenerationFun|NormalizeCoordVector _returnvalue_3)))
    (:then_2
      (bind _returnvalue_5 (Class|ProceduralGenerationActor|CombinationAlgh (Variables|VoronoiDiagram|Getcoef1) _returnvalue_2 (Variables|VoronoiDiagram|Getcoef2) _returnvalue_4 _matrixsize))
      (bind _returnvalue_6 (Class|GenerationFun|NormalizeCoordVector _returnvalue_5)))
    (:then_3
      (bind _output_get (Variables|Default|SetTimeVar (- (+ (Math|Conversions|ToFloat(Integer) _seconds_2) _partialseconds_2) (Variables|Default|GetTimeVar))))
      (return _returnvalue_6 _output_get))))

(fn SetReference
  (params (Painter :type BP%20Height%20Map%20Painter%20Object%20Reference))
  (Utilities|FlowControl|Sequence
    (:then_0
      (bind _returnvalue (Game|SpawnActorfromClass "/Game/StrategyGame/ProceduralGeneration/BP_ProceduralGenerationLandscape.BP_ProceduralGenerationLandscape_C" (Transformation|GetActorTransform self) "Undefined" 0 0))
      (Variables|Reference|SetProceduralGenerationLandscape _returnvalue))
    (:then_1
      (Variables|Reference|SetPainter Painter))))