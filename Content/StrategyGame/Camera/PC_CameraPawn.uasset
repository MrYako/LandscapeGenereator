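; Strategy-game player controller that drives the BP_CameraPawn camera and handles mouse selection input.
; Axis inputs move the pawn at a speed scaled by spring-arm length and Shift; Pan gates mouse rotation with clamped pitch, and zoom adjusts arm length.
; Left-drag toggles MyHUD rectangle drawing; right-click then stores a target location and places a spawned BP_CursorOnPlane along the surface normal.
; Screen-edge scrolling exists but is disconnected.
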(event EventBeginPlay
  (Utilities|FlowControl|Sequence
    (:then_0
      (Utilities|ReferenceCasts))
    (:then_1
      (Utilities|SpawnActorCursor))
    (:then_2
      (bind _asmy_hud (Utilities|Casting|CastToMyHUD (HUD|GetHUD)))
      (Variables|References|SetHUDRef _asmy_hud))))

(event Input|ActionEvents|InputActionPan
  (params (Key :type Key%20Structure))
  (bind _camerapawnref (Variables|References|GetCameraPawnRef))
  (bind _returnvalue (Transformation|GetActorRotation _camerapawnref))
  ;[1 1 1] Pan Y
  (:Pressed
    (Variables|Default|SetDesableCamNav true)
    (Utilities|FlowControl|Gate true) ; enters at Open
  )
  (:Released
    (Variables|Default|SetDesableCamNav false)
    (Utilities|FlowControl|Gate true) ; enters at Close
  ))

(event Input|ActionEvents|InputActionPan
  (params (Key :type Key%20Structure))
  (bind _camerapawnref (Variables|References|GetCameraPawnRef))
  (bind _returnvalue (Transformation|GetActorRotation _camerapawnref))
  ;[1 1 1] Pan X
  (:Pressed
    (Variables|Default|SetDesableCamNav true)
    (Utilities|FlowControl|Gate true) ; enters at Open
  )
  (:Released
    (Variables|Default|SetDesableCamNav false)
    (Utilities|FlowControl|Gate true) ; enters at Close
  ))

(event Input|ActionEvents|InputActionPanReset
  (params (Key :type Key%20Structure))
  (bind _camerapawnref (Variables|References|GetCameraPawnRef))
  (bind _returnvalue (Transformation|GetActorRotation _camerapawnref))
  (bind (_roll _pitch _yaw) (Math|Rotator|BreakRotator _returnvalue))
  ;[1 1 1] PanReset
  (:Pressed
    (Transformation|SetActorRotation (Variables|References|GetCameraPawnRef) (Math|Rotator|MakeRotator _roll 0.0 _yaw))))

(event Input|ActionEvents|InputActionZoomIn
  (params (Key :type Key%20Structure))
  (bind _camerapawnref (Variables|References|GetCameraPawnRef))
  (bind _springarm (Variables|/Game/StrategyGame/Camera/BP_CameraPawn.BP_CameraPawn_C|GetSpringArm _camerapawnref))
  ;[1 1 1] Zoom In/Out
  (:Pressed
    (Variables|/Script/Engine.SpringArmComponent|SetTargetArmLength _springarm (Math|Float|Clamp(Float) (- (Variables|/Script/Engine.SpringArmComponent|GetTargetArmLength _springarm) (Variables|Default|GetZoomSensetivity)) 5e+02 (Variables|Default|GetMaxArmDistance)))))

(event Input|ActionEvents|InputActionZoomOut
  (params (Key :type Key%20Structure))
  (bind _camerapawnref (Variables|References|GetCameraPawnRef))
  (bind _springarm (Variables|/Game/StrategyGame/Camera/BP_CameraPawn.BP_CameraPawn_C|GetSpringArm _camerapawnref))
  ;[1 1 1] Zoom In/Out
  (:Pressed
    (Variables|/Script/Engine.SpringArmComponent|SetTargetArmLength _springarm (Math|Float|Clamp(Float) (+ (Variables|Default|GetZoomSensetivity) (Variables|/Script/Engine.SpringArmComponent|GetTargetArmLength _springarm)) 5e+02 (Variables|Default|GetMaxArmDistance)))))

(event Input|ActionEvents|InputActionZoomReset
  (params (Key :type Key%20Structure))
  ;[1 1 1] Zoom Reset
  (:Pressed
    (Variables|/Script/Engine.SpringArmComponent|SetTargetArmLength (Variables|/Game/StrategyGame/Camera/BP_CameraPawn.BP_CameraPawn_C|GetSpringArm (Variables|References|GetCameraPawnRef)) 1.5e+03)))

(event Input|AxisEvents|InputAxisMoveForward
  (params (AxisValue :type Float%20%28single-precision%29))
  ;[1 1 1] Movement X
  (if (not (Variables|Default|GetDesableCamNav))
    (Transformation|SetActorTransform (Variables|References|GetCameraPawnRef) (Utilities|MovementX (CallFunction|MovementSpeedCalculation) (Variables|Default|GetFastMoveMultiplier) AxisValue (Variables|References|GetCameraPawnRef)))))

(event Input|AxisEvents|InputAxisMoveRight
  (params (AxisValue :type Float%20%28single-precision%29))
  (bind _movesensitivity (CallFunction|MovementSpeedCalculation))
  (bind _fastmovemultiplier (Variables|Default|GetFastMoveMultiplier))
  (bind _camerapawnref (Variables|References|GetCameraPawnRef))
  (bind _transform (Utilities|MovemenY _movesensitivity _fastmovemultiplier AxisValue _camerapawnref))
  (bind (_location _rotation _scale) (Math|Transform|BreakTransform _transform))
  (bind (_x _y) (Math|Vector|BreakVector _location))
  ;[1 1 1] MovementY
  (if (not (Variables|Default|GetDesableCamNav))
    (Transformation|SetActorTransform (Variables|References|GetCameraPawnRef) (Math|Transform|MakeTransform (Math|Vector|MakeVector _x _y 1e+02) _rotation _scale))))

(event Input|MouseEvents|MouseX
  (params (AxisValue :type Float%20%28single-precision%29))
  (bind _camerapawnref (Variables|References|GetCameraPawnRef))
  (bind _returnvalue (Transformation|GetActorRotation _camerapawnref))
  ;[1 1 1] Pan X
  (Utilities|FlowControl|Gate true
    (:Exit
      (Transformation|SetActorRotation (Variables|References|GetCameraPawnRef) (Math|Rotator|MakeRotator (.roll _returnvalue) (.pitch _returnvalue) (+ (.yaw _returnvalue) (* (Variables|Default|GetPanSensitivity) AxisValue)))))))

(event Input|MouseEvents|MouseY
  (params (AxisValue :type Float%20%28single-precision%29))
  (bind _camerapawnref (Variables|References|GetCameraPawnRef))
  (bind _returnvalue (Transformation|GetActorRotation _camerapawnref))
  ;[1 1 1] Pan Y
  (Utilities|FlowControl|Gate true
    (:Exit
      (Transformation|SetActorRotation (Variables|References|GetCameraPawnRef) (Math|Rotator|MakeRotator (.roll _returnvalue) (Math|Float|Clamp(Float) (+ (.pitch _returnvalue) (* (Variables|Default|GetPanSensitivity) AxisValue)) -25.0 25.0) (.yaw _returnvalue))))))

(event Input|MouseEvents|MouseX
  (params (AxisValue :type Float%20%28single-precision%29))
  ;[1 1 1] Edge Movement
)

(event Input|MouseEvents|MouseY
  (params (AxisValue :type Float%20%28single-precision%29))
  ;[1 1 1] Edge Movement
)

(event Input|MouseEvents|LeftMouseButton
  (params (Key :type Key%20Structure))
  (bind _hudref (Variables|References|GetHUDRef))
  ;[1 1 1] Set Rectangle
  (:Pressed
    (Default|StartDraw _hudref)
    (Variables|Default|SetCurTarget false)
    (Rendering|SetVisibility (Variables|/Script/Engine.Actor|GetRootComponent (Variables|References|GetCursorOnPlaneRef)) false false))
  (:Released
    (Default|StopDraw _hudref)
    (Variables|Default|SetSelect true)))

(event Input|MouseEvents|RightMouseButton
  (params (Key :type Key%20Structure))
  (bind _hitresult (Game|Player|GetHitResultUnderCursorbyChannel "TraceTypeQuery1" true))
  (bind _cursoronplaneref (Variables|References|GetCursorOnPlaneRef))
  (bind (_bblockinghit _binitialoverlap _time _distance _location _impactpoint _normal _impactnormal) (Collision|BreakHitResult _hitresult))
  ;[1 1 1] Set Target
  (:Pressed
    (if (Variables|Default|GetSelect)
      (Variables|Default|SetCurTarget true)
      (Variables|Default|SetTargetLoc _location)
      (Rendering|SetVisibility (Variables|/Script/Engine.Actor|GetRootComponent _cursoronplaneref) true false)
      (Transformation|SetActorTransform _cursoronplaneref (Math|Transform|MakeTransform _location (Math|Rotator|MakeRotationfromAxes _impactnormal "0, 0, 0" "0, 0, 0") "1,1,1") true true))))

(event Input|KeyboardEvents|LeftShift
  (params (Key :type Key%20Structure))
  ;[1 1 1] Move Multiplier
  (:Pressed
    (Variables|Default|SetFastMoveMultiplier 4.0))
  (:Released
    (Variables|Default|SetFastMoveMultiplier 1.0)))

(fn ConstructionScript)

(fn MovementSpeedCalculation
  (return (Math|Float|Clamp(Float) (/ (Variables|/Script/Engine.SpringArmComponent|GetTargetArmLength (Variables|/Game/StrategyGame/Camera/BP_CameraPawn.BP_CameraPawn_C|GetSpringArm (Variables|References|GetCameraPawnRef))) 5e+01) 5.0 2e+03)))